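; Combat component that turns attack input into a randomly chosen light attack montage on the owner's mesh.
; ActionInput stores the attack key and consumes it immediately unless IsAttacking is set; nothing here replays a stored key.
; Light attacks set an active state that resets on a timer.
; With movement input held, root motion is briefly ignored at attack start, then re-enabled by timer.
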(event Custom|Action%20Input
  (params (AttackMove :type E_AttackMove%20Enum :default "NewEnumerator0"))
  (bind _output_get (Variables|Default|SetStoredKey AttackMove))
  (if (not (Variables|Default|GetIsAttacking?))
    (CallFunction|ConsumedKey _output_get)
    (Variables|Default|SetStoredKey "NewEnumerator0")))

(event Custom|Consumed%20Key
  (params (Selection :type E_AttackMove%20Enum :default "NewEnumerator0"))
  (switch Utilities|FlowControl|Switch|SwitchonE_AttackMove Selection
    (:NewEnumerator1
      (CallFunction|LightAttack))))

(event Custom|Initialize
  (params (Mesh :type Skeletal%20Mesh%20Component%20Object%20Reference) (CharMovement :type Character%20Movement%20Component%20Object%20Reference))
  (bind _output_get (Variables|Default|SetMesh Mesh))
  (Variables|Default|SetAnimInstance (Components|SkeletalMesh|GetAnimInstance _output_get))
  (Variables|Default|SetChar%20Movement CharMovement))

(fn LightAttack
  (Variables|Default|SetActiveState "NewEnumerator1")
  (CallFunction|IgnoreRootMotion)
  (Animation|Montage|MontagePlay (Variables|Default|GetAnimInstance) (Utilities|Array|Get(acopy) (Variables|Default|GetMontage%20to%20Play) (Math|Random|RandomIntegerinRange 0 1)) 1.0 "MontageLength" 0.0 false)
  (Utilities|Time|SetTimerbyFunctionName 0 "ResetState" 3.0))

(fn IgnoreRootMotion
  (if (Math|Vector|NotEqual(Vector) (Pawn|Components|PawnMovement|GetLastInputVector (Variables|Default|GetChar%20Movement)) "0, 0, 0" 0.0001)
    (Class|AnimInstance|SetRootMotionMode (Variables|Default|GetAnimInstance) "IgnoreRootMotion")
    (Utilities|Time|SetTimerbyFunctionName 0 "EnableRootMotion" 0.3)))

(fn EnableRootMotion
  (Class|AnimInstance|SetRootMotionMode (Variables|Default|GetAnimInstance) "RootMotionFromEverything"))

(fn ResetState
  (Variables|Default|SetActiveState "NewEnumerator0"))