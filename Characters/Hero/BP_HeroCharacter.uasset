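; BP_HeroCharacter is the hero character Blueprint that picks get-up and roll animations and handles held-object update events.
; GetGetUpAnimation branches on whether the ragdoll is face up, then on OverlayState, with some weapon, item and default stances sharing a result.
; GetRollAnimation switches on the same overlay state, grouping only Masculine and Feminine with the default.
; The two held-object events simply forward to their matching On-prefixed calls.
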(event EventUpdateHeldObject
  (CallFunction|OnUpdateHeldObject))

(event EventUpdateHeldObjectAnimations
  (CallFunction|OnUpdateHeldObjectAnimations))

(fn ConstructionScript)

(fn GetGetUpAnimation
  (params (bRagdollFaceUpState :type Boolean))
  (if bRagdollFaceUpState
    (switch Utilities|FlowControl|Switch|SwitchonEALSOverlayState (Variables|Default|GetOverlayState)
      (:Default
        _)
      (:Masculine
        _)
      (:Feminine
        _)
      (:Injured
        (return 0))
      (:HandsTied
        (return 0))
      (:Rifle
        (return 0))
      (:PistolOneHanded
        (return 0))
      (:PistolTwoHanded
        (return 0))
      (:Bow
        (return 0))
      (:Torch
        (return 0))
      (:Binoculars
        (return 0))
      (:Box
        (return 0))
      (:Barrel
        (return 0)))
    (return 0)
    (else
      (switch Utilities|FlowControl|Switch|SwitchonEALSOverlayState (Variables|Default|GetOverlayState)
        (:Default
          _)
        (:Masculine
          _)
        (:Feminine
          _)
        (:Injured
          (return 0))
        (:HandsTied
          (return 0))
        (:Rifle
          (return 0))
        (:PistolOneHanded
          (return 0))
        (:PistolTwoHanded
          (return 0))
        (:Bow
          (return 0))
        (:Torch
          (return 0))
        (:Binoculars
          (return 0))
        (:Box
          (return 0))
        (:Barrel
          (return 0)))
      (return 0))))

(fn GetRollAnimation
  (switch Utilities|FlowControl|Switch|SwitchonEALSOverlayState (Variables|Default|GetOverlayState)
    (:Default
      _)
    (:Masculine
      _)
    (:Feminine
      _)
    (:Injured
      (return 0))
    (:HandsTied
      (return 0))
    (:Rifle
      (return 0))
    (:PistolOneHanded
      (return 0))
    (:PistolTwoHanded
      (return 0))
    (:Bow
      (return 0))
    (:Torch
      (return 0))
    (:Binoculars
      (return 0))
    (:Box
      (return 0))
    (:Barrel
      (return 0)))
  (return 0))