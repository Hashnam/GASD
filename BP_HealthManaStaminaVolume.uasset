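; BP_HealthManaStaminaVolume is a box volume that periodically applies the GE_HealthManaStaminaVolume gameplay effect to characters inside it.
; A looping one-second timer, started on BeginPlay, polls the box's overlapping actors on the authority only.
; Each living GDCharacterBase with a valid Ability System Component applies the effect to itself through a fresh effect context.
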(event Custom|DamageTick
  (Networking|SwitchHasAuthority
    (:Authority
      (for _array_element (Collision|GetOverlappingActors (Variables|Default|GetBox) 0 :!class /Script/Engine.PrimitiveComponent)
        (bind _asgdcharacter_base (Utilities|Casting|CastToGDCharacterBase _array_element))
        (if (and (Class|GDCharacterBase|IsAlive _asgdcharacter_base) (Utilities|IsValid (Ability|GetAbilitySystemComponent _asgdcharacter_base)))
          (GameplayEffects|ApplyGameplayEffectToSelf (Ability|GetAbilitySystemComponent _asgdcharacter_base) "/Game/GASDocumentation/Blueprints/GE_HealthManaStaminaVolume.GE_HealthManaStaminaVolume_C" 1.0 (GameplayEffects|MakeEffectContext (Ability|GetAbilitySystemComponent _asgdcharacter_base))))))))

(event EventBeginPlay
  (Utilities|Time|SetTimerbyEvent (delegate Custom|DamageTick) 1.0 true))

(fn ConstructionScript)